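; BP_Grinder is a rotatable puzzle piece that the player turns to help open the Graveyard_Puzzle_Gate.
; Two trigger boxes set overlap flags, and Tick spins Cylinder2 in opposite directions while the player pawn stays inside either one.
; Near TargetAngle, it destroys both boxes to end rotation, increments the gate's Current count and calls PuzzleComplete.
; An earlier add/remove point scheme and debug prints remain unconnected.
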(event `self.ReceiveTick`
  (params (DeltaSeconds :type "Float (single-precision)"))
  (if (`self.overlappingBox`)
    ;[1 1 1] Rotate in minus dir
    (if (`PrimitiveComponent.IsOverlappingActor` (`self.Box`) (`GameplayStatics.GetPlayerPawn` 0))
      (`SceneComponent.K2_AddLocalRotation` (`self.Cylinder2`) (* (`KismetMathLibrary.MakeRotator` 0.0 0.0 (`self.RotationSpeed`)) -1.0) false false)
      (set `self.CurrentRotation` (`SceneComponent.RelativeRotation` (`self.Cylinder2`)) :!label _label)
      (if (== (`self.CurrentRotation`) (`self.Target_Angle`) :`ErrorTolerance` 5.0)
        (set `self.overlappingBox` false)
        (set `self.overlappingBox1` false)
        (`ActorComponent.K2_DestroyComponent` (`self.Box`))
        (`ActorComponent.K2_DestroyComponent` (`self.Box1`))
        (bind _returnvalue (`GameplayStatics.GetActorOfClass` "/Game/PersonalFolders/Cali/Graveyard_Puzzle_Gate.Graveyard_Puzzle_Gate_C"))
        (set `/Game/PersonalFolders/Cali/Graveyard_Puzzle_Gate.Current` (+ (`/Game/PersonalFolders/Cali/Graveyard_Puzzle_Gate.Current` _returnvalue) 1) _returnvalue)
        (bind _returnvalue_2 (`GameplayStatics.GetActorOfClass` "/Game/PersonalFolders/Cali/Graveyard_Puzzle_Gate.Graveyard_Puzzle_Gate_C"))
        (`/Game/PersonalFolders/Cali/Graveyard_Puzzle_Gate.Puzzle Complete` _returnvalue_2))
      (else
        (set `self.overlappingBox` false)))
    (else
      ;[1 1 1] else check if Overlapping other box THEN rotate
      (if (`self.overlappingBox1`)
        (if (`PrimitiveComponent.IsOverlappingActor` (`self.Box1`) (`GameplayStatics.GetPlayerPawn` 0))
          (`SceneComponent.K2_AddLocalRotation` (`self.Cylinder2`) (* (`KismetMathLibrary.MakeRotator` 0.0 0.0 (`self.RotationSpeed`)) 1.0) false false)
          (goto _label)
          (else
            (set `self.overlappingBox1` false)))))))

(event `self.Box.OnComponentBeginOverlap`
  (params (OverlappedComponent :type "PrimitiveComponent Object Reference") (OtherActor :type "Actor Object Reference") (OtherComp :type "PrimitiveComponent Object Reference") (OtherBodyIndex :type Integer) (bFromSweep :type Boolean) (SweepResult :type "HitResult Structure (by ref)"))
  (set `self.overlappingBox` true))

(event `self.Box1.OnComponentBeginOverlap`
  (params (OverlappedComponent :type "PrimitiveComponent Object Reference") (OtherActor :type "Actor Object Reference") (OtherComp :type "PrimitiveComponent Object Reference") (OtherBodyIndex :type Integer) (bFromSweep :type Boolean) (SweepResult :type "HitResult Structure (by ref)"))
  (set `self.overlappingBox1` true))

(fn `UserConstructionScript`)