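; Player audio component that plays combat, death and magic sounds and handles volume and music-stop events.
; On BeginPlay it binds handlers for those events, drawing cues from InfoAudio, with death and magic reusing the melee cues.
; Melee attacks sphere-trace forward from the capsule, playing the hit cue at the struck actor or the miss cue at the player.
; Stop-music, gated by a bool, calls the ambience actor to stop.
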(event `self.ReceiveBeginPlay`
  (`|ExecutionSequence`
    (:`then_1`
      (add `self.Play-Sfx-Death` (delegate `Death-Sfx`))
      (add `self.Play-Sfx-Cast-Magic` (delegate `Magic-Sfx`))
      (add `self.Assign-Audio-Settings` (delegate `Audio-Settings`))
      (add `self.Stop-Current-Music` (delegate `Stop-Music`))
      (add `self.Sfx-Hit-Enemy` (delegate `Sfx-Hit-Enemy_Event`)))))

(event `Stop-Music`
  (if (`self.Bool-Stop-Music`)
    (bind _asbpa_audio_ambiance (castclass `/Game/Audio/Blueprints/BPA_Audio_Ambiance` "/Game/Audio/Blueprints/BPA_Audio_Ambiance.BPA_Audio_Ambiance_C"))
    (bind _returnvalue (`GameplayStatics.GetActorOfClass` _asbpa_audio_ambiance))
    (`/Game/Audio/Blueprints/BPA_Audio_Ambiance.Stop-Sfx-Play` _returnvalue)))

(event `Death-Sfx` :!signature `self.Play-Sfx-Death`
  (params (Location :type "Vector Structure"))
  (bind (_info_audio_melee_hit _info_audio_melee_no_hit) (break `/Game/Audio/Audio_Components/Structures/Struct_Cue_Player_Combat` (`self.Info_Audio`)))
  (`GameplayStatics.PlaySoundAtLocation` _info_audio_melee_no_hit Location (struct) 1.0 1.0 0.0 null null null))

(event `Audio-Settings` :!signature `self.Assign-Audio-Settings`
  (params (`New-Volume` :type "Float (double-precision)"))
  (set `self.Info-Audio-Settings` (make `/Game/Audio/Blueprints/Struct-Audio-Settings` `New-Volume`)))

(event `Magic-Sfx` :!signature `self.Play-Sfx-Cast-Magic`
  (params (Location :type "Vector Structure"))
  (bind (_info_audio_melee_hit _info_audio_melee_no_hit) (break `/Game/Audio/Audio_Components/Structures/Struct_Cue_Player_Combat` (`self.Info_Audio`)))
  (`GameplayStatics.PlaySoundAtLocation` _info_audio_melee_hit Location (struct) 1.0 1.0 0.0 null null null))

(event `Sfx-Hit-Enemy_Event` :!signature `self.Sfx-Hit-Enemy`
  (params (`Player-Character` :type "/Game/Raccoonik/Art/Characters/ThirdPersonCharacter Object Reference"))
  (bind (_info_audio_melee_hit _info_audio_melee_no_hit) (break `/Game/Audio/Audio_Components/Structures/Struct_Cue_Player_Combat` (`self.Info_Audio`)))
  (bind _capsulecomponent (`Character.CapsuleComponent` `Player-Character`))
  (bind _returnvalue (`SceneComponent.K2_GetComponentLocation` _capsulecomponent))
  ;[0.7706 1 0.99 1 12] Playing the Melee Sound Cue when the Player Character Attacks
  (`KismetSystemLibrary.PrintString` "BPC-Audio-Player has been called... \n__" false false (struct :`R` 1.0 :`G` 0.379183 :`A` 1.0)) ; Debuggin Print String, Currently Disabled..
  (bind (_outhit _returnvalue_2) (`KismetSystemLibrary.SphereTraceSingle` _returnvalue (+ _returnvalue (* (`KismetMathLibrary.GetForwardVector` (`SceneComponent.K2_GetComponentRotation` _capsulecomponent)) 100.0)) 50.0 "TraceTypeQuery1")) ; Sphere Trace checks to see if the player has struck something,\ndepending on the return a different sound will be played.
  (if _returnvalue_2
    ;;[1 0.3604 0 1 10] Debugging Print Strings, Disabled may need in Future...
    (`GameplayStatics.PlaySoundAtLocation` _info_audio_melee_hit (`Actor.K2_GetActorLocation` (`.HitActor` (`GameplayStatics.BreakHitResult` _outhit))) (struct) 1.0 1.0 0.0 null null null) ; Playing Sound Cue of the Player \nHitting Something.
    (`KismetSystemLibrary.PrintString` "Audio Line Trace Returned as True \n__" false false (struct :`R` 1.0 :`G` 0.277368 :`A` 1.0))
    (else
      (`GameplayStatics.PlaySoundAtLocation` _info_audio_melee_no_hit (`Actor.K2_GetActorLocation` `Player-Character`) (struct) 1.0 1.0 0.0 null null null) ; Playing Sound Cue of the Player \nNOT Hitting Something.
      (`KismetSystemLibrary.PrintString` "Audio Line Trace Returned as False \n__" false false (struct :`R` 1.0 :`G` 0.416046 :`A` 1.0)))))