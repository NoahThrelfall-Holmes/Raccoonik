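; BP_Ladder is a climbable ladder with a configurable height.
; The construction script stacks mesh segments from LadderHeight and LadderUnitHeight and sizes the trigger box to fit.
; When a ThirdPersonCharacter enters the box, a short forward trace checks that it faces the ladder before calling the ClimbLadder dispatcher.
; Leaving the box restores Walking movement and clears the character's IsClimbing flag.
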(event `self.TriggerBox.OnComponentBeginOverlap`
  (params (OverlappedComponent :type "PrimitiveComponent Object Reference") (OtherActor :type "Actor Object Reference") (OtherComp :type "PrimitiveComponent Object Reference") (OtherBodyIndex :type Integer) (bFromSweep :type Boolean) (SweepResult :type "HitResult Structure (by ref)"))
  (bind _asthird_person_character (cast `/Game/Raccoonik/Art/Characters/ThirdPersonCharacter` OtherActor))
  (bind _returnvalue (`self.K2_GetActorLocation` _asthird_person_character))
  (bind _outhit (`KismetSystemLibrary.LineTraceSingle` :`Start` _returnvalue :`End` (+ _returnvalue (* (`self.GetActorForwardVector` _asthird_person_character) 100)) :`TraceChannel` "TraceTypeQuery1" :`bIgnoreSelf` false))
  (if (== (`.HitActor` (`GameplayStatics.BreakHitResult` _outhit)) self)
    (`self.Climb Ladder`)))

(event `self.TriggerBox.OnComponentEndOverlap`
  (params (OverlappedComponent :type "PrimitiveComponent Object Reference") (OtherActor :type "Actor Object Reference") (OtherComp :type "PrimitiveComponent Object Reference") (OtherBodyIndex :type Integer))
  (bind _asthird_person_character (cast `/Game/Raccoonik/Art/Characters/ThirdPersonCharacter` OtherActor))
  (`CharacterMovementComponent.SetMovementMode` (`Character.CharacterMovement` _asthird_person_character) "MOVE_Walking" 0)
  (set `/Game/Raccoonik/Art/Characters/ThirdPersonCharacter.IsClimbing` false _asthird_person_character))

(fn `UserConstructionScript`
  (bind _ladderunitheight (`self.LadderUnitHeight`))
  (bind _ladderunitheight_2 (`self.LadderUnitHeight`))
  (bind _ladderunitheight_3 (`self.LadderUnitHeight`))
  (bind _triggerbox (`self.TriggerBox`))
  (for _index (range (+ (`self.LadderHeight`) 1))
    (`AddComponent|NODE_AddStaticMeshComponent-0` :`RelativeTransform` (`KismetMathLibrary.MakeTransform` (`KismetMathLibrary.MakeVector` 0.0 0.0 (+ (* _index _ladderunitheight_3) _ladderunitheight_3)) (struct :`Yaw` -90.0)))
    (`SceneComponent.K2_SetRelativeLocation` _triggerbox (`KismetMathLibrary.MakeVector` 40.0 0.0 (+ (* (/ (`self.LadderHeight`) 2) _ladderunitheight) (* 3 _ladderunitheight))) false false)
    (`BoxComponent.SetBoxExtent` _triggerbox (`KismetMathLibrary.MakeVector` 40.0 60.0 (+ (/ (* (`self.LadderHeight`) _ladderunitheight_2) 2.0) _ladderunitheight_2)) true)))