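; Lock-on indicator actor that shows a widget above the enemy nearest the player.
; Each Tick, while unlocked, it searches actors of a class, stores the nearest within tracking distance as the lock target, and otherwise hides the widget and clears the target.
; While ThirdPersonCharacter is locked on, the widget stays over the stored enemy.
; A target change briefly hides the widget, using a short delay to restart its animation.
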(event `self.ReceiveTick`
  (params (DeltaSeconds :type "Float (single-precision)"))
  (bind _returnvalue (`self.GetTransform` (`self.NearestEnemy`)))
  (bind _returnvalue_2 (`self.GetTransform` (`self.NearestEnemy`)))
  ;[1 1 1] finding enemys and displaying target on them
  (bind _asthird_person_character (cast `/Game/Raccoonik/Art/Characters/ThirdPersonCharacter` (`GameplayStatics.GetPlayerCharacter` 0)))
  (if (`/Game/Raccoonik/Art/Characters/ThirdPersonCharacter.LockedOn` _asthird_person_character)
    (`SceneComponent.K2_SetWorldLocation` (`self.LockOnWidget`) (`KismetMathLibrary.MakeVector` (.x (.location _returnvalue_2)) (.y (.location _returnvalue_2)) (+ (.z (.location _returnvalue_2)) 100.0)) false false) ; place widget over enemy
    (else
      (bind _outactors (`GameplayStatics.GetAllActorsOfClass` null)) ; Get all actors in a class \n(eventually there will be an enemyclass that holds this data)
      (bind (_distance _returnvalue_3) (`GameplayStatics.FindNearestActor` (`self.K2_GetActorLocation` (`GameplayStatics.GetPlayerPawn` 0)) _outactors))
      (if (< _distance (`KismetMathLibrary.Conv_IntToDouble` (`self.LockTrackingDistance`)))
        (if (!= _returnvalue_3 (`self.NearestEnemy`))
          (`SceneComponent.SetVisibility` (`self.LockOnWidget`) false false) ; to reset animations
        )
        (set `self.NearestEnemy` _returnvalue_3)
        (`SceneComponent.K2_SetWorldLocation` (`self.LockOnWidget`) (`KismetMathLibrary.MakeVector` (.x (.location _returnvalue)) (.y (.location _returnvalue)) (+ (.z (.location _returnvalue)) 100.0)) false false) ; place widget over enemy
        (set `self.ObjectLockTarget` (`self.NearestEnemy`))
        (`KismetSystemLibrary.Delay` 0.1) ; so the animation can reset\n(doesn't work without this)
        (`SceneComponent.SetVisibility` (`self.LockOnWidget`) true false)
        (else
          (`SceneComponent.SetVisibility` (`self.LockOnWidget`) false false) ; if not, make widget invisible
          (set `self.ObjectLockTarget` null))))))

(fn `UserConstructionScript`)