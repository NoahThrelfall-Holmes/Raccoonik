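; BP_Potion is a consumable potion that restores the player's mana or health.
; Its Consume event plays DrinkingAnimation on the ThirdPersonCharacter mesh and, without waiting for the montage to finish, switches on PotionType.
; Mana and Health call ManaHeal or Heal on player 0's character with the truncated Value, while a Null type prints a fault message.
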(event `Consume`
  (bind _returnvalue (`GameplayStatics.GetPlayerCharacter` 0))
  (bind _returnvalue_2 (`KismetMathLibrary.FTrunc` (`self.Value`)))
  (bind _asthird_person_character (cast `/Game/Raccoonik/Art/Characters/ThirdPersonCharacter` (`GameplayStatics.GetPlayerCharacter` 0)))
  (`|PlayMontage` (`Character.Mesh` _asthird_person_character) (`self.DrinkingAnimation`)
    (:`then`
      (switch `/Game/Raccoonik/Core/misc/EPotionType` (`self.PotionType`)
        (:`NewEnumerator2`
          (`KismetSystemLibrary.PrintString` "Fault: BP_Potion: Potion Type = Null"))
        (:`NewEnumerator0`
          (bind _asthird_person_character_2 (cast `/Game/Raccoonik/Art/Characters/ThirdPersonCharacter` _returnvalue))
          (`Entity.ManaHeal` _asthird_person_character_2 _returnvalue_2))
        (:`NewEnumerator1`
          (bind _asthird_person_character_3 (cast `/Game/Raccoonik/Art/Characters/ThirdPersonCharacter` _returnvalue))
          (`Entity.Heal` _asthird_person_character_3 _returnvalue_2))))))

(fn `UserConstructionScript`)